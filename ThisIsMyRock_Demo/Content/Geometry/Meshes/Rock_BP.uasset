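; A physics rock that can be picked up and thrown, and calls Bumped on characters it hits when either is moving fast, sparing the thrower.
; RockData sets its scale and mass on BeginPlay, with a random starting rotation.
; Hits spawn bump and fall impact effects, throttled by gates with short delays.
; Tick halves custom time dilation while overlapping water and round-trips the actor transform through CurrentTransform.
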(event `self.ReceiveHit`
  (params (MyComp :type "PrimitiveComponent Object Reference") (Other :type "Actor Object Reference") (OtherComp :type "PrimitiveComponent Object Reference") (bSelfMoved :type Boolean) (HitLocation :type "Vector Structure") (HitNormal :type "Vector Structure") (NormalImpulse :type "Vector Structure") (Hit :type "HitResult Structure (by ref)"))
  (bind _returnvalue (`KismetMathLibrary.VSize` (`self.GetVelocity`)))
  (bind _returnvalue_2 (`KismetMathLibrary.VSize` (`self.GetVelocity`)))
  (bind _returnvalue_3 (`KismetMathLibrary.FClamp` _returnvalue_2 1.0 3.0))
  (bind _asthird_person_character (cast `/Game/ThirdPersonBP/Blueprints/ThirdPersonCharacter` Other)
    (:`then`
      (bind _returnvalue_4 (`KismetMathLibrary.VSize` (`self.GetVelocity` _asthird_person_character)))
      (`KismetSystemLibrary.PrintString` (`KismetStringLibrary.Concat_StrStr` (`KismetStringLibrary.Conv_DoubleToString` _returnvalue_4) "/" (`KismetStringLibrary.Conv_DoubleToString` _returnvalue)))
      (if (not (== Other (`self.ThrowRef`)))
        (set `self.ThrowRef` null)
        (if (or (> _returnvalue_4 300.0) (> _returnvalue 300.0))
          (`/Game/ThirdPersonBP/Blueprints/ThirdPersonCharacter.Bumped` _asthird_person_character)
          (`KismetSystemLibrary.PrintString` "BUMPED" true true (struct :`R` 1.0 :`G` 0.038177 :`A` 1.0))
          ;[1 1 1] VFX cooldown
          (`/Engine/EditorBlueprintResources/StandardMacros.Gate` false :!label _label
            (:`Exit`
              (bind _returnvalue_5 (`KismetMathLibrary.VSize` (`self.GetVelocity` _asthird_person_character)))
              (bind _returnvalue_6 (`KismetMathLibrary.FClamp` _returnvalue_5 1.0 3.0))
              (`GameplayStatics.SpawnEmitterAtLocation` "/Game/Geometry/Particles/BumpImpact.BumpImpact" HitLocation (struct) (select `bool` (> _returnvalue_5 _returnvalue_2) :`false` (`KismetMathLibrary.MakeVector` _returnvalue_3 _returnvalue_3 _returnvalue_3) :`true` (`KismetMathLibrary.MakeVector` _returnvalue_6 _returnvalue_6 _returnvalue_6)))
              (`|ExecutionSequence`
                (:`then_0`
                  (goto _label :!via `Close`))
                (:`then_1`
                  ;[1 0.176 0.2158] thai code
                  (`GameplayStatics.SpawnEmitterAtLocation` "/Game/Geometry/Particles/FallImpact.FallImpact" HitLocation (struct) (* (`SceneComponent.K2_GetComponentScale` (`self.StaticMesh`)) 0.6) :!label _label_2)
                  (`|ExecutionSequence`
                    (:`then_0`
                      (goto _label_3 :!via `Close`))
                    (:`then_1`
                      (`KismetSystemLibrary.Delay` 0.2)
                      (goto _label_3 :!via `Open`))))
                (:`then_2`
                  (`KismetSystemLibrary.Delay` 0.2)
                  (goto _label :!via `Open`)))))
          (else
            (`/Engine/EditorBlueprintResources/StandardMacros.Gate` false :!label _label_3
              (:`Exit`
                (if (not (== (`self.GetVelocity`) (0.0 0.0 0.0) :`ErrorTolerance` 100.0))
                  (goto _label_2))))))))
    (:`CastFailed`
      (set `self.ThrowRef` null)
      (goto _label_3))))

(event `self.ReceiveBeginPlay`
  (bind _staticmesh (`self.StaticMesh`))
  (bind (_rockname _rockscore _rocksize) (break `/Game/Geometry/Meshes/Rock_Struct` (`self.RockData`)))
  (`SceneComponent.SetWorldScale3D` _staticmesh (* (1.0 1.0 1.0) _rocksize))
  (`PrimitiveComponent.SetMassOverrideInKg` _staticmesh "None" (* _rocksize 100.0) true)
  (`self.SetPhysicsSim` (`self.EnablePhysics`))
  (`SceneComponent.K2_SetWorldRotation` (`self.StaticMesh`) (`KismetMathLibrary.RandomRotator` true) false false))

(event `SetPhysicsSim`
  (params (NewValue :type Boolean))
  (`PrimitiveComponent.SetSimulatePhysics` (`self.StaticMesh`) NewValue))

(event `GetCurrentTransform`
  (set `self.CurrentTransform` (`self.GetTransform`)))

(event `ApplyTransform`
  (`self.K2_SetActorTransform` (`self.CurrentTransform`)))

(event `PickedUp`
  (params (Character :type "/Game/ThirdPersonBP/Blueprints/ThirdPersonCharacter Object Reference"))
  (set `self.Carrier` Character)
  (`/Engine/EditorBlueprintResources/StandardMacros.IsValid` Character
    (:`Is Valid`
      (set `self.ThrowRef` Character))))

(event `self.ReceiveTick`
  (params (DeltaSeconds :type "Float (single-precision)"))
  ;[1 0.2344 0.2344] thai code
  (set `self.CustomTimeDilation` (select `bool` (>= (`KismetArrayLibrary.Array_Length` (`PrimitiveComponent.GetOverlappingActors` (`self.StaticMesh`) "/Game/ThirdPersonBP/Blueprints/Water_BP.Water_BP_C")) 1) :`false` 1.0 :`true` 0.5 :!type "Float (single-precision)"))
  (`self.GetCurrentTransform`)
  (`self.ApplyTransform`))

(fn `UserConstructionScript`)